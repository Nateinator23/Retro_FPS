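; First-person player character with axis-driven movement, mouse look and an equipped weapon.
; On BeginPlay it adds WBP_HUD to the viewport and equips BP_PlayerWeaponBase through the Weapon child actor component.
; Equipping swaps the child actor class, sends an init message via IPlayerWeapon and plays the weapon's draw sequence.
; Tick casts the child actor and drives its weapon bob from whether the character is moving.
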(event `InputAxis|HorizontalMovement`
  (params (AxisValue :type "Float (single-precision)"))
  (bind (_returnvalue_roll _returnvalue_pitch _returnvalue_yaw) (`KismetMathLibrary.BreakRotator` (`self.GetControlRotation`)))
  ;[1 1 1] movement
  (`self.AddMovementInput` (`KismetMathLibrary.GetRightVector` (`KismetMathLibrary.MakeRotator` 0.0 0.0 _returnvalue_yaw)) AxisValue))

(event `self.ReceiveBeginPlay`
  (bind _returnvalue (`|CreateWidget` "/Game/BluePrints/WBP_HUD.WBP_HUD_C"))
  (`UserWidget.AddToViewport` _returnvalue 0)
  (`self.EquipWeapon` "/Game/BluePrints/BP_PlayerWeaponBase.BP_PlayerWeaponBase_C"))

(event `InputAxis|VerticalMovement`
  (params (AxisValue :type "Float (single-precision)"))
  (bind (_returnvalue_roll _returnvalue_pitch _returnvalue_yaw) (`KismetMathLibrary.BreakRotator` (`self.GetControlRotation`)))
  ;[1 1 1] movement
  (`self.AddMovementInput` (`KismetMathLibrary.GetForwardVector` (`KismetMathLibrary.MakeRotator` 0.0 0.0 _returnvalue_yaw)) AxisValue))

(event `EquipWeapon`
  (params (Weapon :type "/Game/BluePrints/BP_PlayerWeaponBase Class Reference"))
  (bind _weapon (`self.weapon`))
  (bind _childactor (`ChildActorComponent.ChildActor` _weapon))
  ;[1 1 1] Equp weapon
  (bind _output_get (set `self.CurrentWeapon` Weapon))
  (`ChildActorComponent.SetChildActorClass` _weapon _output_get)
  (if (`KismetSystemLibrary.DoesImplementInterface` _childactor "/Game/BluePrints/IPlayerWeapon.IPlayerWeapon_C")
    (message `/Game/BluePrints/IPlayerWeapon.Initi_Weapon` _childactor)
    (bind _asbp_player_weapon_base (cast `/Game/BluePrints/BP_PlayerWeaponBase` _childactor))
    (`MovieSceneSequencePlayer.Play` (`ActorSequenceComponent.SequencePlayer` (`/Game/BluePrints/BP_PlayerWeaponBase.Weapon Draaw` _asbp_player_weapon_base)))))

(event `InputAxis|MouseLookHorizontal`
  (params (AxisValue :type "Float (single-precision)"))
  ;[1 1 1] mouse look
  (`self.AddControllerYawInput` AxisValue))

(event `InputAxis|MouseLookVertical`
  (params (AxisValue :type "Float (single-precision)"))
  ;[1 1 1] mouse look
  (`self.AddControllerPitchInput` AxisValue))

(event `self.ReceiveTick`
  (params (DeltaSeconds :type "Float (single-precision)"))
  (bind _asbp_player_weapon_base (cast `/Game/BluePrints/BP_PlayerWeaponBase` (`ChildActorComponent.ChildActor` (`self.weapon`))))
  (`/Game/BluePrints/BP_PlayerWeaponBase.WeaponBob` _asbp_player_weapon_base (> (`KismetMathLibrary.VSize` (`MovementComponent.Velocity` (`self.CharacterMovement`))) 0.0) DeltaSeconds))

(fn `UserConstructionScript`)