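; Upgrade station actor that opens an upgrade menu when the player interacts with it.
; BeginPlay creates the Upgrade_UI widget and adds it to the viewport; HeagneyInteract makes it visible, shows the cursor, disables OnRailsCharacter movement, pauses the game and switches to UI-only input.
; Tick yaw-billboards the Paper sprite toward the camera.
; Player overlap with the box only prints a welcome message, and the Interact event is empty.
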(event `self.ReceiveBeginPlay`
  ;[1 1 1] Begin Play
  (bind _returnvalue (`|CreateWidget` "/Game/OnRails/Ui/Upgrade_UI.Upgrade_UI_C"))
  (bind _output_get (set `self.UpgradeWidget` _returnvalue))
  (`UserWidget.AddToViewport` _output_get 1))

(event `/Game/OnRails/BP_Interface.heagneyInteract`
  (bind _returnvalue (`GameplayStatics.GetPlayerController` 0))
  ;[1 1 1] Interaction
  (set `PlayerController.bShowMouseCursor` true _returnvalue)
  (`Widget.SetVisibility` (`self.UpgradeWidget`) "Visible")
  (bind _ason_rails_character (cast `/Game/OnRails/OnRailsCharacter` (`GameplayStatics.GetPlayerCharacter` 0)))
  (set `/Game/OnRails/OnRailsCharacter.CanMove?` false _ason_rails_character)
  (`GameplayStatics.SetGamePaused` true)
  (`WidgetBlueprintLibrary.SetInputMode_UIOnlyEx` _returnvalue null)
  (`GameplayStatics.PlaySound2D` null 1.0 1.0 0.0 null null))

(event `self.ReceiveTick`
  (params (DeltaSeconds :type "Float (single-precision)"))
  (bind _papersprite (`self.PaperSprite`))
  (bind (_returnvalue_roll _returnvalue_pitch _returnvalue_yaw) (`KismetMathLibrary.BreakRotator` (`KismetMathLibrary.FindLookAtRotation` (`SceneComponent.K2_GetComponentLocation` _papersprite) (`PlayerCameraManager.GetCameraLocation` (`GameplayStatics.GetPlayerCameraManager` 0)))))
  ;[1 1 1] TICK (I know its bad)
  (`SceneComponent.K2_SetWorldRotation` _papersprite (`KismetMathLibrary.MakeRotator` 0.0 0.0 (- _returnvalue_yaw 90.0)) false false))

(event `/Game/OnRails/BP_Interface.Interact`)

(event `self.Box.OnComponentBeginOverlap`
  (params (OverlappedComponent :type "PrimitiveComponent Object Reference") (OtherActor :type "Actor Object Reference") (OtherComp :type "PrimitiveComponent Object Reference") (OtherBodyIndex :type Integer) (bFromSweep :type Boolean) (SweepResult :type "HitResult Structure (by ref)"))
  (if (== OtherActor (`GameplayStatics.GetPlayerCharacter` 0))
    (`KismetSystemLibrary.PrintString` "Welcome")))

(fn `UserConstructionScript`)