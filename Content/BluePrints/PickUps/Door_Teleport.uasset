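; Interactable teleport door that moves the player to another level.
; On HeagneyInteract it passes TeleportStage to the OnRails character, shows a Fade widget and starts a looping timer that steadily narrows the camera FOV as a zoom-in.
; After a short delay it calls GetCharacterStats on the game instance and opens the level named by LevelName.
; The timer-clear and FOV-reset nodes are unconnected and never run.
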(event `self.ReceiveBeginPlay`
  (`PaperSpriteComponent.SetSprite` (`self.PaperSprite`) (`self.SpriteDoor`)))

(event `/Game/OnRails/BP_Interface.heagneyInteract`
  (bind _ason_rails_character (cast `/Game/OnRails/OnRailsCharacter` (`GameplayStatics.GetPlayerCharacter` 0)))
  (set `self.As on Rails Character` _ason_rails_character)
  (set `/Game/OnRails/OnRailsCharacter.TeleportStage` (`self.Teleport Stage`) _ason_rails_character)
  (bind _returnvalue (`|CreateWidget` "/Game/OnRails/Ui/Fade.Fade_C"))
  (`UserWidget.AddToViewport` _returnvalue 0)
  (`UserWidget.PlayAnimation` _returnvalue (`/Game/OnRails/Ui/Fade.Fade` _returnvalue) 0.0 1 "Forward" 1.0 false)
  (`self.add FOV`)
  (`KismetSystemLibrary.Delay` 0.5)
  (`self.Rest`))

(event `add FOV`
  (bind _output_get (set `self.FOV` (- (`self.FOV`) 0.1)))
  (`CameraComponent.SetFieldOfView` (`/Game/OnRails/OnRailsCharacter.Camera` (`self.As on Rails Character`)) _output_get)
  (bind _returnvalue (`KismetSystemLibrary.K2_SetTimerDelegate` (delegate `add FOV`) 0.01 true))
  (set `self.NewVar` _returnvalue))

(event `Rest`
  (bind _asgame_stats_bp (cast `/Game/GameStats_BP` (`GameplayStatics.GetGameInstance`)))
  (`/Game/GameStats_BP.GetCharacterStats` _asgame_stats_bp)
  (`GameplayStatics.OpenLevel` (`self.Level Name`)))

(fn `UserConstructionScript`)