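; Gun pickup Blueprint that gives the on-rails player the rifle when they walk into it.
; When the player character overlaps its box, it reveals the rifle and energy widget on OnRailsCharacter and enables right-click.
; It then spawns a pickup particle effect, plays a 2D pickup sound and destroys itself.
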(event `self.Box.OnComponentBeginOverlap`
  (params (OverlappedComponent :type "PrimitiveComponent Object Reference") (OtherActor :type "Actor Object Reference") (OtherComp :type "PrimitiveComponent Object Reference") (OtherBodyIndex :type Integer) (bFromSweep :type Boolean) (SweepResult :type "HitResult Structure (by ref)"))
  (bind _returnvalue (`GameplayStatics.GetPlayerCharacter` 0))
  (if (== OtherActor _returnvalue)
    (bind _ason_rails_character (cast `/Game/OnRails/OnRailsCharacter` _returnvalue))
    (`SceneComponent.SetVisibility` (`/Game/OnRails/OnRailsCharacter.Rifle` _ason_rails_character) true false)
    (`SceneComponent.SetVisibility` (`/Game/OnRails/OnRailsCharacter.EnergyWidget` _ason_rails_character) true false)
    (set `/Game/OnRails/OnRailsCharacter.CanRightClick?` true _ason_rails_character)
    (`NiagaraFunctionLibrary.SpawnSystemAtLocation` "/Game/Particle/GunEffects/Pickup_Res.Pickup_Res" (`self.K2_GetActorLocation`))
    (`GameplayStatics.PlaySound2D` "/Game/OnRails/Sounds/Pickup/PickUP_Cue.PickUP_Cue" 1.0 1.0 0.0 null null)
    (`self.K2_DestroyActor`)))

(fn `UserConstructionScript`)