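; KeyCard is a pickup actor that raises the player's access level.
; When the player character overlaps its Box component, it adds one to AccessLevel on OnRailsCharacter and then destroys itself.
; A node that would set the Cube component's mesh to MeshKeyCard exists but is not connected, and the construction script is empty.
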(event `self.ReceiveBeginPlay`)

(event `self.Box.OnComponentBeginOverlap`
  (params (OverlappedComponent :type "PrimitiveComponent Object Reference") (OtherActor :type "Actor Object Reference") (OtherComp :type "PrimitiveComponent Object Reference") (OtherBodyIndex :type Integer) (bFromSweep :type Boolean) (SweepResult :type "HitResult Structure (by ref)"))
  (bind _returnvalue (`GameplayStatics.GetPlayerCharacter` 0))
  (bind _ason_rails_character (cast `/Game/OnRails/OnRailsCharacter` _returnvalue :!pure true))
  (if (== OtherActor _returnvalue)
    (set `/Game/OnRails/OnRailsCharacter.Access Level` (+ (`/Game/OnRails/OnRailsCharacter.Access Level` _ason_rails_character) 1) _ason_rails_character)
    (`self.K2_DestroyActor`)))

(fn `UserConstructionScript`)