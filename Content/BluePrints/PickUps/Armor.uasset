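; Armor pickup actor that restores armor to the OnRailsCharacter that overlaps its box.
; On overlap it adds HealValue to the character's Armor, capped at MaxArmor, then briefly flashes a widget on the viewport.
; The DestroyActor node is unconnected, so the graph never removes the pickup after use.
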(event `self.Box.OnComponentBeginOverlap`
  (params (OverlappedComponent :type "PrimitiveComponent Object Reference") (OtherActor :type "Actor Object Reference") (OtherComp :type "PrimitiveComponent Object Reference") (OtherBodyIndex :type Integer) (bFromSweep :type Boolean) (SweepResult :type "HitResult Structure (by ref)"))
  (bind _as_on_rails_character (`self.As on Rails Character`))
  (bind _as_on_rails_character_2 (`self.As on Rails Character`))
  (bind _returnvalue (+ (`/Game/OnRails/OnRailsCharacter.Armor` _as_on_rails_character) (`self.Heal Value`)))
  (bind _ason_rails_character (cast `/Game/OnRails/OnRailsCharacter` OtherActor))
  (set `self.As on Rails Character` _ason_rails_character)
  (if (>= _returnvalue (`/Game/OnRails/OnRailsCharacter.MaxArmor` _as_on_rails_character))
    (set `/Game/OnRails/OnRailsCharacter.Armor` (`/Game/OnRails/OnRailsCharacter.MaxArmor` _as_on_rails_character_2) _as_on_rails_character_2)
    (else
      (set `/Game/OnRails/OnRailsCharacter.Armor` _returnvalue _as_on_rails_character_2)))
  (bind _returnvalue_2 (`|CreateWidget` "/Game/OnRails/Ui/Armor.Armor_C"))
  (bind _output_get (set `self.ArmorWidget` _returnvalue_2))
  (`UserWidget.AddToViewport` _output_get 0)
  (`KismetSystemLibrary.Delay` 0.1)
  (`Widget.RemoveFromParent` _returnvalue_2))

(fn `UserConstructionScript`)