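; Breakable crate actor that drops a RecourcePickUp when destroyed.
; AnyDamage sets Health to incoming Damage minus current Health (operands reversed from a usual decrement), then tests for zero or below.
; On that condition it spawns a break particle system, plays a 2D crate-break sound, spawns the pickup at its own transform and destroys itself.
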(event `self.ReceiveAnyDamage`
  (params (Damage :type "Float (single-precision)") (DamageType :type "DamageType Object Reference") (InstigatedBy :type "Controller Object Reference") (DamageCauser :type "Actor Object Reference"))
  (set `self.Health` (- Damage (`self.Health`)))
  (if (<= (`self.Health`) 0.0)
    (`NiagaraFunctionLibrary.SpawnSystemAtLocation` "/Game/Particle/GunEffects/BulletHit_Break.BulletHit_Break" (`self.K2_GetActorLocation`))
    (`GameplayStatics.PlaySound2D` "/Game/OnRails/Sounds/Break/66777__kevinkace__crate-break-1_Cue.66777__kevinkace__crate-break-1_Cue" 1.0 1.0 0.0 null null)
    (`|SpawnActorFromClass` "/Game/BluePrints/PickUps/RecourcePickUp.RecourcePickUp_C" (`self.GetTransform`) "Undefined" "MultiplyWithRoot" null null)
    (`self.K2_DestroyActor`)))

(fn `UserConstructionScript`)