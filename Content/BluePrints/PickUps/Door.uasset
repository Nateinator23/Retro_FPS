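; Door pickup-folder Blueprint that slides open once for a player with sufficient access.
; When the player character overlaps the Box, it compares the OnRailsCharacter's AccessLevel to DoorLevel.
; A passing check goes through a DoOnce, stores the start location and plays the MoveDoor timeline, lerping the whole actor 500 units along world X.
; Nothing resets or closes it; two duplicate access checks are left unconnected.
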(event `self.Box.OnComponentBeginOverlap`
  (params (OverlappedComponent :type "PrimitiveComponent Object Reference") (OtherActor :type "Actor Object Reference") (OtherComp :type "PrimitiveComponent Object Reference") (OtherBodyIndex :type Integer) (bFromSweep :type Boolean) (SweepResult :type "HitResult Structure (by ref)"))
  (bind _returnvalue (`GameplayStatics.GetPlayerCharacter` 0))
  (if (== OtherActor _returnvalue)
    (if (>= (`/Game/OnRails/OnRailsCharacter.Access Level` (cast `/Game/OnRails/OnRailsCharacter` _returnvalue :!pure true)) (`self.DoorLevel`))
      (`/Engine/EditorBlueprintResources/StandardMacros.DoOnce` false
        (:`Completed`
          (set `self.Start Location` (`self.K2_GetActorLocation`))
          (bind (_direction _new) (`Timeline|Move Door` :!via `PlayFromStart`)
            (:`Update`
              (`self.K2_SetActorLocation` (`KismetMathLibrary.VLerp` (`self.Start Location`) (+ (`self.Start Location`) (500.0 0.0 0.0)) _new)))))))))

(fn `UserConstructionScript`)