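; HealthMachine is an interactable machine that opens an upgrade menu and pauses the game.
; On BeginPlay it creates the Upgrade_UI widget and adds it to the viewport.
; Interact shows the cursor and widget, turns off GunMove on the OnRailsCharacter, pauses, and switches to UI-only input.
; Closing the menu is not handled here, and the music-spawning nodes are unconnected.
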(event `self.ReceiveBeginPlay`
  (bind _returnvalue (`|CreateWidget` "/Game/OnRails/Ui/Upgrade_UI.Upgrade_UI_C"))
  (bind _output_get (set `self.UpgradeWidget` _returnvalue))
  (`UserWidget.AddToViewport` _output_get 0))

(event `/Game/OnRails/BP_Interface.Interact`
  (bind _returnvalue (`GameplayStatics.GetPlayerController` 0))
  (set `PlayerController.bShowMouseCursor` true _returnvalue)
  (`Widget.SetVisibility` (`self.UpgradeWidget`) "Visible")
  (bind _ason_rails_character (cast `/Game/OnRails/OnRailsCharacter` (`GameplayStatics.GetPlayerCharacter` 0)))
  (set `/Game/OnRails/OnRailsCharacter.GunMove?` false _ason_rails_character)
  (`GameplayStatics.SetGamePaused` true)
  (`WidgetBlueprintLibrary.SetInputMode_UIOnlyEx` _returnvalue null))

(fn `UserConstructionScript`)