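; Shooting range target that moves between two points and awards score when damaged.
; The construction script builds InterpToMovement's relative path from two location variables and sets its duration.
; On BeginPlay, the sphere takes its configured material and scale.
; Any damage adds Amount to the Score on the ORC_ShootingRange player character, then destroys the target, provided that cast succeeds.
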(event `self.ReceiveBeginPlay`
  (bind _sphere (`self.Sphere`))
  (`PrimitiveComponent.SetMaterial` _sphere 0 (`self.Material`))
  (`SceneComponent.SetRelativeScale3D` _sphere (`self.New Scale 3D`)))

(event `self.ReceiveAnyDamage`
  (params (Damage :type "Float (single-precision)") (DamageType :type "DamageType Object Reference") (InstigatedBy :type "Controller Object Reference") (DamageCauser :type "Actor Object Reference"))
  (bind _asorc_shooting_range (cast `/Game/OnRails/ORC_ShootingRange` (`GameplayStatics.GetPlayerCharacter` 0)))
  (set `/Game/OnRails/ORC_ShootingRange.Score` (+ (`/Game/OnRails/ORC_ShootingRange.Score` _asorc_shooting_range) (`self.Amount`)) _asorc_shooting_range)
  (`self.K2_DestroyActor`))

(fn `UserConstructionScript`
  (bind _interptomovement (`self.InterpToMovement`))
  (set `InterpToMovementComponent.ControlPoints` (`|MakeArray` (make `InterpControlPoint` (`self.Location1`)) (make `InterpControlPoint` (`self.Location2`))) _interptomovement)
  (set `InterpToMovementComponent.Duration` (`self.Duration`) _interptomovement))