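; Alarm actor that pulses a point light and plays an alarm sound in an endless loop from BeginPlay.
; The Rest event runs two timelines in sequence, Fade then Timeline, each driving the light's intensity.
; Alarm_Cue plays at the actor's location as each timeline finishes, and the second one calls Rest again to restart the cycle.
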(event `self.ReceiveBeginPlay`
  (`self.Rest`))

(event `Rest`
  (bind (_direction _newtrack_0) (`Timeline|Fade` :!via `PlayFromStart`)
    (:`Update`
      (`LightComponent.SetIntensity` (`self.PointLight`) _newtrack_0))
    (:`Finished`
      (`GameplayStatics.PlaySoundAtLocation` "/Game/Sounds/Alarm_Cue.Alarm_Cue" (`self.K2_GetActorLocation`) (struct) 1.0 1.0 0.0 null null null null)
      (bind (_direction_2 _newtrack_0_2) (`Timeline|Timeline` :!via `PlayFromStart`)
        (:`Update`
          (`LightComponent.SetIntensity` (`self.PointLight`) _newtrack_0_2))
        (:`Finished`
          (`GameplayStatics.PlaySoundAtLocation` "/Game/Sounds/Alarm_Cue.Alarm_Cue" (`self.K2_GetActorLocation`) (struct) 1.0 1.0 0.0 null null null null)
          (`self.Rest`))))))

(fn `UserConstructionScript`)