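; BP_Fade is a trigger volume that plays a one-time screen fade when the player character enters its box.
; The first player overlap sets the OnRailsCharacter camera's field of view to 90 and creates a Fade widget playing its FadingOUT animation.
; The widget is removed from the screen after a short fixed delay, and the DoOnce is never reset.
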(event `self.Box.OnComponentBeginOverlap`
  (params (OverlappedComponent :type "PrimitiveComponent Object Reference") (OtherActor :type "Actor Object Reference") (OtherComp :type "PrimitiveComponent Object Reference") (OtherBodyIndex :type Integer) (bFromSweep :type Boolean) (SweepResult :type "HitResult Structure (by ref)"))
  (if (== OtherActor (`GameplayStatics.GetPlayerCharacter` 0))
    (`/Engine/EditorBlueprintResources/StandardMacros.DoOnce` false
      (:`Completed`
        (bind _ason_rails_character (cast `/Game/OnRails/OnRailsCharacter` (`GameplayStatics.GetPlayerCharacter` 0)))
        (`CameraComponent.SetFieldOfView` (`/Game/OnRails/OnRailsCharacter.Camera` _ason_rails_character) 90.0)
        (bind _returnvalue (`|CreateWidget` "/Game/OnRails/Ui/Fade.Fade_C"))
        (`UserWidget.AddToViewport` _returnvalue 0)
        (`UserWidget.PlayAnimation` _returnvalue (`/Game/OnRails/Ui/Fade.FadingOUT` _returnvalue) 0.0 1 "Forward" 1.0 false)
        (`KismetSystemLibrary.Delay` 0.6)
        (`Widget.RemoveFromParent` _returnvalue)))))

(fn `UserConstructionScript`)