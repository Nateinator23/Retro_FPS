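; Elevator actor that moves its Cube platform when the player character enters a trigger Box.
; Overlap plays the MovingElevator timeline, which lerps the Cube's relative location from the origin to the configurable NewRelativeLocation without sweeping.
; When the player leaves the Box, the timeline reverses to return the platform only if WantToGoBackUp is set.
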(event `self.Box.OnComponentBeginOverlap`
  (params (OverlappedComponent :type "PrimitiveComponent Object Reference") (OtherActor :type "Actor Object Reference") (OtherComp :type "PrimitiveComponent Object Reference") (OtherBodyIndex :type Integer) (bFromSweep :type Boolean) (SweepResult :type "HitResult Structure (by ref)"))
  (if (== OtherActor (`GameplayStatics.GetPlayerCharacter` 0))
    (bind (_direction _newtrack_1) (`Timeline|MovingElevator` :!label _label)
      (:`Update`
        (`SceneComponent.K2_SetRelativeLocation` (`self.Cube`) (`KismetMathLibrary.VLerp` (0.0 0.0 0.0) (`self.New Relative Location`) _newtrack_1) false false)))))

(event `self.Box.OnComponentEndOverlap`
  (params (OverlappedComponent :type "PrimitiveComponent Object Reference") (OtherActor :type "Actor Object Reference") (OtherComp :type "PrimitiveComponent Object Reference") (OtherBodyIndex :type Integer))
  (if (== OtherActor (`GameplayStatics.GetPlayerCharacter` 0))
    (if (`self.Want to go back up?`)
      (goto _label :!via `Reverse`))))

(fn `UserConstructionScript`)