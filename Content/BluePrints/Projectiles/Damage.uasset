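; Damage volume Blueprint that drains the player's Health while something overlaps its Box component.
; Begin overlap calls Damaging, which subtracts Health from player 0's OnRailsCharacter and re-arms a looping timer on itself for repeated ticks.
; End overlap clears that timer.
; Neither overlap event checks the overlapping actor, so any overlap damages the player.
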(event `Damaging`
  ;[1 0 0.761] Damaging
  (bind _ason_rails_character (cast `/Game/OnRails/OnRailsCharacter` (`GameplayStatics.GetPlayerCharacter` 0)))
  (set `/Game/OnRails/OnRailsCharacter.Health` (- (`/Game/OnRails/OnRailsCharacter.Health` _ason_rails_character) 1.0) _ason_rails_character)
  (bind _returnvalue (`KismetSystemLibrary.K2_SetTimer` null "Damaging" 0.1 true))
  (set `self.Timer` _returnvalue))

(event `self.Box.OnComponentBeginOverlap`
  (params (OverlappedComponent :type "PrimitiveComponent Object Reference") (OtherActor :type "Actor Object Reference") (OtherComp :type "PrimitiveComponent Object Reference") (OtherBodyIndex :type Integer) (bFromSweep :type Boolean) (SweepResult :type "HitResult Structure (by ref)"))
  ;[1 0.3906 0.3906] Overlap
  (`self.Damaging`))

(event `self.Box.OnComponentEndOverlap`
  (params (OverlappedComponent :type "PrimitiveComponent Object Reference") (OtherActor :type "Actor Object Reference") (OtherComp :type "PrimitiveComponent Object Reference") (OtherBodyIndex :type Integer))
  ;[1 0.3906 0.3906] Overlap
  (`KismetSystemLibrary.K2_ClearAndInvalidateTimerHandle` (`self.Timer`)))

(fn `UserConstructionScript`)