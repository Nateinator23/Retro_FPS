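; Base player weapon Blueprint that displays a 2D flipbook weapon with movement bob.
; A SceneCaptureComponent2D is restricted to the WeaponFlipbook, isolating the weapon render from the world.
; InitiWeapon calls SetFlipbook and hides the flipbook in game.
; The WeaponBob event plays a sequence while moving; otherwise it stops it and interpolates the flipbook back to the relative location cached at BeginPlay.
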(event `self.ReceiveBeginPlay`
  (`SceneCaptureComponent.ShowOnlyComponent` (`self.SceneCaptureComponent2D`) (`self.WeaponFlipbook`))
  (set `self.WeaponPosition` (`SceneComponent.RelativeLocation` (`self.WeaponFlipbook`))))

(event `/Game/BluePrints/IPlayerWeapon.Initi_Weapon`
  (bind _weaponflipbook (`self.WeaponFlipbook`))
  (`PaperFlipbookComponent.SetFlipbook` _weaponflipbook null)
  (`SceneComponent.SetHiddenInGame` _weaponflipbook true false))

(event `WeaponBob`
  (params (IsMoving :type Boolean) (`Dealta Time` :type "Float (double-precision)"))
  (bind _weaponflipbook (`self.WeaponFlipbook`))
  (bind _sequenceplayer (`ActorSequenceComponent.SequencePlayer` (`self.Weapon Bob`)))
  (if IsMoving
    (`MovieSceneSequencePlayer.Play` _sequenceplayer)
    (else
      (`MovieSceneSequencePlayer.Stop` _sequenceplayer)
      (`SceneComponent.K2_SetRelativeLocation` _weaponflipbook (`KismetMathLibrary.VInterpTo` (`SceneComponent.RelativeLocation` _weaponflipbook) (`self.WeaponPosition`) `Dealta Time` 10.0) false false))))

(fn `UserConstructionScript`)