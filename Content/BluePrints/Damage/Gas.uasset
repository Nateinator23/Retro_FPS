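; Gas hazard volume for the on-rails player that erodes maximum health while they stand inside it and shows a Radiation widget.
; Box overlap starts a looping one-second Damaging timer that applies damage, subtracts it from MaxHealth down to a threshold and clamps Health to match.
; Leaving clears the timer and widget, then restores MaxHealth to MaxMaxHealth after a short delay if the player has not re-entered.
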(event `Damaging`
  (bind _as_on_rails_character (`self.As on Rails Character`))
  (bind _maxhealth (`/Game/OnRails/OnRailsCharacter.MaxHealth` _as_on_rails_character))
  ;[1 1 1] Damage
  (bind _ason_rails_character (cast `/Game/OnRails/OnRailsCharacter` (`GameplayStatics.GetPlayerCharacter` 0)))
  (bind _output_get (set `self.As on Rails Character` _ason_rails_character))
  (if (not (<= (`/Game/OnRails/OnRailsCharacter.MaxHealth` (`self.As on Rails Character`)) 25.0))
    (bind _returnvalue (`GameplayStatics.ApplyDamage` _output_get (`self.Base Damage`)))
    (set `/Game/OnRails/OnRailsCharacter.MaxHealth` (- (`/Game/OnRails/OnRailsCharacter.MaxHealth` _output_get) _returnvalue) _as_on_rails_character)
    (if (> (`/Game/OnRails/OnRailsCharacter.Health` _as_on_rails_character) _maxhealth)
      (set `/Game/OnRails/OnRailsCharacter.Health` _maxhealth _as_on_rails_character))
    (bind _returnvalue_2 (`KismetSystemLibrary.K2_SetTimer` null "Damaging" 1.0 true))
    (set `self.Timer` _returnvalue_2)))

(event `self.Box.OnComponentBeginOverlap`
  (params (OverlappedComponent :type "PrimitiveComponent Object Reference") (OtherActor :type "Actor Object Reference") (OtherComp :type "PrimitiveComponent Object Reference") (OtherBodyIndex :type Integer) (bFromSweep :type Boolean) (SweepResult :type "HitResult Structure (by ref)"))
  ;[1 1 1] Begin
  (bind _ason_rails_character (cast `/Game/OnRails/OnRailsCharacter` OtherActor))
  (if (== _ason_rails_character OtherActor)
    (set `self.IsIn?` true)
    (`self.Damaging`)
    (bind _returnvalue (`|CreateWidget` "/Game/OnRails/Ui/Radiation.Radiation_C"))
    (bind _output_get (set `self.RadWidget` _returnvalue))
    (`UserWidget.AddToViewport` _output_get 0)))

(event `self.Box.OnComponentEndOverlap`
  (params (OverlappedComponent :type "PrimitiveComponent Object Reference") (OtherActor :type "Actor Object Reference") (OtherComp :type "PrimitiveComponent Object Reference") (OtherBodyIndex :type Integer))
  (bind _as_on_rails_character (`self.As on Rails Character`))
  ;[1 1 1] End
  (`KismetSystemLibrary.K2_ClearAndInvalidateTimerHandle` (`self.Timer`))
  (`Widget.RemoveFromParent` (`self.RadWidget`))
  (set `self.IsIn?` false)
  (`KismetSystemLibrary.Delay` 3.0)
  (if (not (`self.IsIn?`))
    (set `/Game/OnRails/OnRailsCharacter.MaxHealth` (`/Game/OnRails/OnRailsCharacter.MaxMaxHealth` _as_on_rails_character) _as_on_rails_character)))

(fn `UserConstructionScript`)