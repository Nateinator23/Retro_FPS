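; GameStats_BP holds a copy of the player's OnRailsCharacter stats so they can be saved off and restored later.
; GetCharacterStats copies health, weapon, energy, resource, access level, kill count and other values from player character 0 into its own variables.
; RecoverPlayerStats writes the same values back onto the current player character.
; Both events are plain field-by-field copies that stop if the cast to OnRailsCharacter fails.
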(event `GetCharacterStats`
  (bind _as_on_rails_character (`self.As on Rails Character`))
  (bind _ason_rails_character (cast `/Game/OnRails/OnRailsCharacter` (`GameplayStatics.GetPlayerCharacter` 0)))
  (set `self.As on Rails Character` _ason_rails_character)
  (set `self.Health` (`/Game/OnRails/OnRailsCharacter.Health` _as_on_rails_character))
  (set `self.FireRate` (`/Game/OnRails/OnRailsCharacter.FireRate` _as_on_rails_character))
  (set `self.MaxHealth` (`/Game/OnRails/OnRailsCharacter.MaxHealth` _as_on_rails_character))
  (set `self.Base Damage` (`/Game/OnRails/OnRailsCharacter.Base Damage` _as_on_rails_character))
  (set `self.Resource` (`/Game/OnRails/OnRailsCharacter.Resource` _as_on_rails_character))
  (set `self.Access Level` (`/Game/OnRails/OnRailsCharacter.Access Level` _as_on_rails_character))
  (set `self.MaxMaxHealth` (`/Game/OnRails/OnRailsCharacter.MaxMaxHealth` _as_on_rails_character))
  (set `self.RadiationHealth` (`/Game/OnRails/OnRailsCharacter.RadiationHealth` _as_on_rails_character))
  (set `self.Scale Value` (`/Game/OnRails/OnRailsCharacter.Scale Value` _as_on_rails_character))
  (set `self.Enemy Kills` (`/Game/OnRails/OnRailsCharacter.Enemy Kills` _as_on_rails_character))
  (set `self.EnergyAmount` (`/Game/OnRails/OnRailsCharacter.EnergyAmount` _as_on_rails_character))
  (set `self.EnergyUsage` (`/Game/OnRails/OnRailsCharacter.EnergyUsage` _as_on_rails_character))
  (set `self.EnergyRechargeRate` (`/Game/OnRails/OnRailsCharacter.EnergyRechargeRate` _as_on_rails_character))
  (set `self.EnergyRechargeTimer` (`/Game/OnRails/OnRailsCharacter.EnergyRechargeTimer` _as_on_rails_character))
  (set `self.EnergyMax` (`/Game/OnRails/OnRailsCharacter.EnergyMax` _as_on_rails_character))
  (set `self.Ammo` (`/Game/OnRails/OnRailsCharacter.Ammo` _as_on_rails_character))
  (set `self.ChanceOfEffect` (`/Game/OnRails/OnRailsCharacter.ChanceOfEffect` _as_on_rails_character))
  (set `self.GunEffect` (`/Game/OnRails/OnRailsCharacter.GunEffect` _as_on_rails_character)))

(event `RecoverPlayerStats`
  (bind _ason_rails_character (cast `/Game/OnRails/OnRailsCharacter` (`GameplayStatics.GetPlayerCharacter` 0)))
  (set `/Game/OnRails/OnRailsCharacter.Health` (`self.Health`) _ason_rails_character)
  (set `/Game/OnRails/OnRailsCharacter.FireRate` (`self.FireRate`) _ason_rails_character)
  (set `/Game/OnRails/OnRailsCharacter.MaxHealth` (`self.MaxHealth`) _ason_rails_character)
  (set `/Game/OnRails/OnRailsCharacter.Base Damage` (`self.Base Damage`) _ason_rails_character)
  (set `/Game/OnRails/OnRailsCharacter.Resource` (`self.Resource`) _ason_rails_character)
  (set `/Game/OnRails/OnRailsCharacter.Access Level` (`self.Access Level`) _ason_rails_character)
  (set `/Game/OnRails/OnRailsCharacter.MaxMaxHealth` (`self.MaxMaxHealth`) _ason_rails_character)
  (set `/Game/OnRails/OnRailsCharacter.RadiationHealth` (`self.RadiationHealth`) _ason_rails_character)
  (set `/Game/OnRails/OnRailsCharacter.Scale Value` (`self.Scale Value`) _ason_rails_character)
  (set `/Game/OnRails/OnRailsCharacter.Enemy Kills` (`self.Enemy Kills`) _ason_rails_character)
  (set `/Game/OnRails/OnRailsCharacter.EnergyAmount` (`self.EnergyAmount`) _ason_rails_character)
  (set `/Game/OnRails/OnRailsCharacter.EnergyUsage` (`self.EnergyUsage`) _ason_rails_character)
  (set `/Game/OnRails/OnRailsCharacter.EnergyRechargeRate` (`self.EnergyRechargeRate`) _ason_rails_character)
  (set `/Game/OnRails/OnRailsCharacter.EnergyRechargeTimer` (`self.EnergyRechargeTimer`) _ason_rails_character)
  (set `/Game/OnRails/OnRailsCharacter.EnergyMax` (`self.EnergyMax`) _ason_rails_character)
  (set `/Game/OnRails/OnRailsCharacter.Ammo` (`self.Ammo`) _ason_rails_character)
  (set `/Game/OnRails/OnRailsCharacter.ChanceOfEffect` (`self.ChanceOfEffect`) _ason_rails_character)
  (set `/Game/OnRails/OnRailsCharacter.GunEffect` (`self.GunEffect`) _ason_rails_character))