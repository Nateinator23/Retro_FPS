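; BP_NPC is an NPC Blueprint that opens a dialog UI when its OnDialog event fires.
; The event creates a Dialog_Widget for the passed-in player, adds it to the viewport, switches input to UI-only and prints a debug greeting.
; It binds the widget's OnExit dispatcher, which restores Game-and-UI input for the owning player and removes the widget.
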(event `/Game/Dialog/Interact_Dialog.OnDialog`
  (params (Character :type "/Game/OnRails/OnRailsController Object Reference"))
  (bind _returnvalue (`|CreateWidget` "/Game/Dialog/UI/Dialog_Widget.Dialog_Widget_C" Character))
  (bind _output_get (set `self.NewVar` _returnvalue))
  (add `/Game/Dialog/UI/Dialog_Widget.OnExit` _output_get (delegate `OnExit_Event`))
  (`UserWidget.AddToViewport` _output_get 0)
  (`WidgetBlueprintLibrary.SetInputMode_UIOnlyEx` Character _output_get)
  (`KismetSystemLibrary.PrintString` "Hello"))

(event `OnExit_Event`
  (`WidgetBlueprintLibrary.SetInputMode_GameAndUIEx` (`Widget.GetOwningPlayer` (`self.NewVar`)) null)
  (`Widget.RemoveFromParent` (`self.NewVar`)))

(fn `UserConstructionScript`)